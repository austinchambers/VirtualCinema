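; BP_Blui is an actor that shows a web page on an in-world plane using the BLUI browser plugin.
; On BeginPlay it creates a BluEye, sets it to load the Unreal Engine site as an opaque view, and initializes it.
; The browser's material instance, based on HTMLMat, is then applied to DisplayPlane.
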(event `self.ReceiveBeginPlay`
  (bind _ui1 (`self.UI1`))
  (set `self.UI1` (`BluBlueprintFunctionLibrary.NewBluEye`))
  (set `BluEye.DefaultURL` "http://unrealengine.com" _ui1)
  (set `BluEye.BaseMaterial` "/Game/Materials/HTMLMat.HTMLMat" _ui1)
  (set `BluEye.bEnabled` true _ui1)
  (set `BluEye.bIsTransparent` false _ui1)
  (`BluEye.init` _ui1)
  (`PrimitiveComponent.SetMaterial` (`self.DisplayPlane`) 0 (`BluEye.GetMaterialInstance` _ui1)))

(event `self.ReceiveActorBeginOverlap`
  (params (OtherActor :type "Actor Object Reference")))

(event `self.ReceiveTick`
  (params (DeltaSeconds :type "Float (single-precision)")))

(fn `UserConstructionScript`)