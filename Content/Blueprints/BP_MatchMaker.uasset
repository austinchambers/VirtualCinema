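; BP_MatchMaker is an actor that automatically matchmakes LAN multiplayer as soon as play begins.
; It searches for LAN sessions and joins the first one found, printing whether the join succeeded.
; If none are found, it creates a four-slot session and opens MultiplayerLevel1 as a listen server.
; Search and session-creation failures are not handled.
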(event `self.ReceiveBeginPlay`
  (bind _returnvalue (`GameplayStatics.GetPlayerController` 0))
  (bind _results (`FindSessionsCallbackProxy.FindSessions` (`GameplayStatics.GetPlayerController` 0) 4 true)
    (:`OnSuccess`
      (if (== (`KismetArrayLibrary.Array_Length` _results) 0)
        (`CreateSessionCallbackProxy.CreateSession` _returnvalue 4 true
          (:`OnSuccess`
            (`GameplayStatics.OpenLevel` "MultiplayerLevel1" true "listen")))
        (else
          (`JoinSessionCallbackProxy.JoinSession` _returnvalue (`KismetArrayLibrary.Array_Get` _results)
            (:`OnSuccess`
              (`KismetSystemLibrary.PrintString` "Join Success"))
            (:`OnFailure`
              (`KismetSystemLibrary.PrintString` "Join Failed"))))))))

(event `self.ReceiveActorBeginOverlap`
  (params (OtherActor :type "Actor Object Reference")))

(event `self.ReceiveTick`
  (params (DeltaSeconds :type "Float (single-precision)")))

(fn `UserConstructionScript`)